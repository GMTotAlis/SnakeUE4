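; Food actor that steps through colored stages after spawning, lowering its score value the longer it exists.
; BeginPlay starts SetFood at Blue, which swaps the mesh and material, sets Score, waits, then calls itself with the next type.
; The chain runs through Purple and Red with progressively shorter delays, and stops at Yellow, the lowest-value stage.
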(event `self.ReceiveBeginPlay`
  (`self.Set Food` "NewEnumerator0"))

(event `Set Food`
  (params (Type :type "/Game/Blueprint/FoodColor_Enum Enum" :default "NewEnumerator0"))
  (bind _food_mesh (`self.Food Mesh`))
  (switch `/Game/Blueprint/FoodColor_Enum` Type
    (:`NewEnumerator0`
      (`StaticMeshComponent.SetStaticMesh` _food_mesh "/Engine/BasicShapes/Cube.Cube")
      (`PrimitiveComponent.SetMaterial` _food_mesh 0 "/Game/Materials/Blue_M.Blue_M")
      (set `self.Score` 100)
      (`KismetSystemLibrary.Delay` 3.0)
      (`self.Set Food` "NewEnumerator1"))
    (:`NewEnumerator1`
      (`StaticMeshComponent.SetStaticMesh` _food_mesh "/Engine/BasicShapes/Cone.Cone")
      (`PrimitiveComponent.SetMaterial` _food_mesh 0 "/Game/Materials/Purple_M.Purple_M")
      (set `self.Score` 50)
      (`KismetSystemLibrary.Delay` 2.0)
      (`self.Set Food` "NewEnumerator2"))
    (:`NewEnumerator2`
      (`StaticMeshComponent.SetStaticMesh` _food_mesh "/Engine/BasicShapes/Cylinder.Cylinder")
      (`PrimitiveComponent.SetMaterial` _food_mesh 0 "/Game/Materials/Red_M.Red_M")
      (set `self.Score` 20)
      (`KismetSystemLibrary.Delay` 1.5)
      (`self.Set Food` "NewEnumerator3"))
    (:`NewEnumerator3`
      (`StaticMeshComponent.SetStaticMesh` _food_mesh "/Engine/EngineMeshes/MaterialSphere.MaterialSphere")
      (`PrimitiveComponent.SetMaterial` _food_mesh 0 "/Game/Materials/Yellow_M.Yellow_M")
      (set `self.Score` 10))))

(fn `UserConstructionScript`)